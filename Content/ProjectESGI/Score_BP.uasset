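; Score_BP is an actor that keeps a score and shows it through a text render.
; On BeginPlay it finds the Timer_BP actor in the level and stores a reference to it.
; AddScoreText adds points only while that timer is active, then refreshes the displayed text.
; ResetText sets the score back to zero and updates the display through the same text update.
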(event Custom|AddScoreText
  (params (Points :type Integer))
  (if (Variables|/Game/ProjectESGI/Timer_BP.Timer_BP_C|GetIsTimerActive (Variables|Default|GetTimerRef))
    (bind _output_get (Variables|Default|SetScore (+ (Variables|Default|GetScore) Points)))
    (Rendering|Components|TextRender|SetText (Variables|Default|GetTextRender) (Utilities|Text|ToText(Integer) (stale Custom|ResetText _output_get)))))

(event Custom|ResetText
  (bind _output_get (Variables|Default|SetScore 0))
  (Rendering|Components|TextRender|SetText (Variables|Default|GetTextRender) (Utilities|Text|ToText(Integer) _output_get)))

(event EventBeginPlay
  (bind _returnvalue (Actor|GetActorOfClass "/Game/ProjectESGI/Timer_BP.Timer_BP_C"))
  (Variables|Default|SetTimerRef _returnvalue))

(fn ConstructionScript)