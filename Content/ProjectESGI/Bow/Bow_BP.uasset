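; Grabbable-string bow that loads an arrow and fires it with force based on draw distance.
; Tick projects the held string grab point onto the segment between two spline points, storing draw as a normalized ratio, and snaps it back when not held.
; An Arrow_BP entering the box is destroyed and replaced by a visible dummy arrow.
; Releasing the string while loaded launches an Arrow_Projectile, hides the dummy and tells the ArrowSpawner to spawn.
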(event OnComponentBeginOverlap(Box)
  (params (OverlappedComponent :type Primitive%20Component%20Object%20Reference) (OtherActor :type Actor%20Object%20Reference) (OtherComp :type Primitive%20Component%20Object%20Reference) (OtherBodyIndex :type Integer) (bFromSweep :type Boolean) (SweepResult :type Hit%20Result%20Structure%20%28by%20ref%29))
  (bind _asarrow_bp (Utilities|Casting|CastToArrow_BP OtherActor))
  (if (not (Variables|Default|GetIsLoaded))
    (Variables|Default|SetIsLoaded true)
    (Development|SetHiddeninGame (Variables|Default|GetArrow) false false)
    (Actor|DestroyActor _asarrow_bp)))

(event OnDropped(StringGrabComponent)
  (bind _arrowforspawn (Variables|Default|GetArrowForSpawn))
  (bind _grabactor (Variables|Default|GetGrabActor))
  (Variables|Default|SetForce (* (Variables|Default|GetCurrent%20Slider%20Value) (Variables|Default|GetMultiplicator)))
  (Transformation|SetWorldRotation _grabactor (Transformation|GetWorldRotation (Variables|Default|GetSpline)) false false)
  (Physics|SetSimulatePhysics _grabactor false)
  (Variables|Default|SetCurrent%20Slider%20Value 0.0)
  (if (Variables|Default|GetIsLoaded)
    (bind _returnvalue (Game|SpawnActorfromClass "/Game/ProjectESGI/Arrow/Arrow_Projectile.Arrow_Projectile_C" (Transformation|GetWorldTransform _arrowforspawn) "Undefined" "MultiplyWithRoot" 0 0))
    (Default|SetSpeed _returnvalue (Variables|Default|GetForce) (Math|Vector|GetForwardVector _arrowforspawn))
    (Development|SetHiddeninGame (Variables|Default|GetArrow) true false)
    (Variables|Default|SetIsLoaded false)
    (bind _returnvalue_2 (Actor|GetActorOfClass "/Game/ProjectESGI/ArrowSpawner.ArrowSpawner_C"))
    (Default|Spawn _returnvalue_2)))

(event EventBeginPlay
  (Development|SetHiddeninGame (Variables|Default|GetArrow) true false))

(event EventTick
  (params (DeltaSeconds :type Float%20%28single-precision%29))
  (bind _stringgrabcomponent (Variables|Default|GetStringGrabComponent))
  (bind _spline (Variables|Default|GetSpline))
  (bind _returnvalue (Transformation|GetWorldLocation _stringgrabcomponent))
  (bind _returnvalue_2 (Spline|GetLocationatSplinePoint _spline 1 "World"))
  (bind _returnvalue_3 (Spline|GetLocationatSplinePoint _spline 0 "World"))
  (bind _returnvalue_4 (Math|Vector|FindClosestPointonSegment _returnvalue _returnvalue_3 _returnvalue_2))
  (Transformation|SetWorldRotation (Variables|Default|GetGrabActor) (Transformation|GetWorldRotation (Variables|Default|GetSpline)) false false)
  (Utilities|IsValid _stringgrabcomponent
    (:Is%20Valid
      (if (Variables|/Game/VRTemplate/Blueprints/GrabComponent.GrabComponent_C|GetbIsHeld _stringgrabcomponent)
        (Variables|Default|SetCurrent%20Slider%20Value (/ (Math|Vector|Distance(Vector) _returnvalue_4 _returnvalue_3) (Math|Vector|Distance(Vector) _returnvalue_2 _returnvalue_3)))
        (Transformation|SetWorldLocation (Variables|Default|GetGrabActor) _returnvalue_4 false false)
        (else
          (Transformation|SetWorldLocation (Variables|Default|GetGrabActor) (Spline|GetLocationatSplinePoint (Variables|Default|GetSpline) 0 "World") false true))))))

(fn ConstructionScript)