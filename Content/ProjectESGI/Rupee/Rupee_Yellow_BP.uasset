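; Yellow rupee target that awards points when hit by an arrow, apparently for a shooting gallery.
; An Arrow_Projectile overlapping the Box plays a bell sound and adds Points to the Score_BP found in the level.
; Instead of being destroyed, the Rupee component teleports to a far-off position, then returns to its saved start position after RespawnTime.
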(event OnComponentBeginOverlap(Box)
  (params (OverlappedComponent :type Primitive%20Component%20Object%20Reference) (OtherActor :type Actor%20Object%20Reference) (OtherComp :type Primitive%20Component%20Object%20Reference) (OtherBodyIndex :type Integer) (bFromSweep :type Boolean) (SweepResult :type Hit%20Result%20Structure%20%28by%20ref%29))
  (Utilities|Casting|CastToArrow_Projectile OtherActor)
  (Audio|PlaySoundatLocation "/Game/ProjectESGI/OOT_ShootingGallery_Bell.OOT_ShootingGallery_Bell" (Transformation|GetWorldLocation (Variables|Default|GetRupee)) "0, 0, 0" 1.0 1.0 0.0 0 0 0 0)
  (bind _returnvalue (Actor|GetActorOfClass "/Game/ProjectESGI/Score_BP.Score_BP_C"))
  (Default|AddScoreText _returnvalue (Variables|Default|GetPoints))
  (Transformation|SetWorldLocation (Variables|Default|GetRupee) "-1000.000000,-1000.000000,-1000.000000" false true)
  (Utilities|FlowControl|Delay (Variables|Default|GetRespawnTime))
  (Transformation|SetWorldLocation (Variables|Default|GetRupee) (Variables|Default|GetStartPosition) false true))

(event EventBeginPlay
  (Variables|Default|SetStartPosition (Transformation|GetWorldLocation (Variables|Default|GetRupee))))

(fn ConstructionScript)